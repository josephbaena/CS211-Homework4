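; BP_Door is an interactive door that the player opens and closes by pressing F or the left gamepad face button.
; Overlapping its trigger box enables input from player controller 0, and leaving disables it.
; Each press flips the DoorStatus boolean and plays or reverses the DoorRotation timeline, whose track drives the actor's relative yaw.
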(event OnComponentBeginOverlap(TriggerBox)
  (params (OtherActor :type Actor%20Object%20Reference) (OtherComp :type Primitive%20Component%20Object%20Reference) (OtherBodyIndex :type Integer) (bFromSweep :type Boolean) (SweepResult :type Hit%20Result%20Structure%20%28by%20ref%29))
  (Input|EnableInput (Game|GetPlayerController 0)))

(event OnComponentEndOverlap(TriggerBox)
  (params (OtherActor :type Actor%20Object%20Reference) (OtherComp :type Primitive%20Component%20Object%20Reference) (OtherBodyIndex :type Integer))
  (Input|DisableInput (Game|GetPlayerController 0)))

(event EventBeginPlay)

(event EventActorBeginOverlap
  (params (OtherActor :type Actor%20Object%20Reference)))

(event EventTick
  (params (DeltaSeconds :type Float%20%28single-precision%29)))

(event Input|KeyboardEvents|F
  (:Pressed
    (if (Variables|Default|GetDoorStatus)
      (Variables|Default|SetDoorStatus false)
      (bind _doorrotation (Timeline|DoorRotation Play)
        (:Update
          (Transformation|SetActorRelativeRotation (Class|KismetMathLibrary|MakeRot 0.0 _doorrotation 0.0))))
      (else
        (Variables|Default|SetDoorStatus true)
        (Timeline|DoorRotation Reverse)))))

(event Input|GamepadEvents|GamepadFaceButtonLeft
  (:Pressed
    (if (Variables|Default|GetDoorStatus)
      (Variables|Default|SetDoorStatus false)
      (bind _doorrotation (Timeline|DoorRotation Play)
        (:Update
          (Transformation|SetActorRelativeRotation (Class|KismetMathLibrary|MakeRot 0.0 _doorrotation 0.0))))
      (else
        (Variables|Default|SetDoorStatus true)
        (Timeline|DoorRotation Reverse)))))

(fn ConstructionScript)